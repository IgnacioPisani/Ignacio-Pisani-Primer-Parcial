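; BP_Enemigos is an enemy actor that moves along its local axes and can fire bullets.
; Tick adds VelocidadEnemigo as a local offset each frame, without sweep or delta-time scaling.
; A looping timer set on BeginPlay calls Disparar, which spawns BP_Bala at the actor's transform when DisparaEnemigo is true.
; Two setter functions expose the velocity and the firing flag.
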(event Custom|Disparar
  (if (Variables|Propiedades|GetbDisparaEnemigo)
    (CallFunction|SpawnearBala)))

(event EventBeginPlay
  (Utilities|Time|SetTimerbyEvent (delegate Custom|Disparar) 0.0 true))

(event Collision|EventActorBeginOverlap
  (params (OtherActor :type Actor%20Object%20Reference)))

(event EventTick
  (params (DeltaSeconds :type Float%20%28single-precision%29))
  (Transformation|AddActorLocalOffset (Variables|Propiedades|GetVelocidadEnemigo) false false))

(fn ConstructionScript)

(fn SetearVelocidadEnemigo
  (params (VelocidadEnemigo :type Vector))
  (Variables|Propiedades|SetVelocidadEnemigo VelocidadEnemigo))

(fn SetearDispara
  (params (bDispara :type Boolean))
  (Variables|Propiedades|SetbDisparaEnemigo bDispara))

(fn SpawnearBala
  (Game|SpawnActorfromClass "/Game/Blueprints/BP_Bala.BP_Bala_C" (Transformation|GetActorTransform) "Undefined" "MultiplyWithRoot" 0 "0.000000,0.000000,0.000000" 0))