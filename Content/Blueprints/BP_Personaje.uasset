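; BP_Personaje is an actor that moves constantly along a local direction and speeds up while flagged as being followed.
; BeginPlay builds the velocity from a normalized editable vector times a factor; Tick applies it as an unswept offset, unscaled by delta time.
; A looping timer checks the flag, set through SetearEstaSiendoSeguido, then doubles velocity after a delay, compounding on later checks, with debug prints.
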(event Custom|Chequear
  (if (Variables|Propiedades|GetbEstaSiendoSeguido)
    (Development|PrintString (Utilities|String|ToString(Vector) (Variables|Propiedades|GetVelocidad)) true true "(R=0.000000,G=0.660000,B=1.000000,A=1.000000)" 1e+01)
    (Utilities|FlowControl|Delay (Variables|Propiedades|GetTiempoDuplicarVel))
    (Variables|Propiedades|SetVelocidad (* (Variables|Propiedades|GetVelocidad) 2.0))
    (Development|PrintString (Utilities|String|ToString(Vector) (Variables|Propiedades|GetVelocidad)) true true "(R=0.000000,G=0.660000,B=1.000000,A=1.000000)" 1e+01)))

(event EventBeginPlay
  (Variables|Propiedades|SetVelocidad (* (Math|Vector|Normalize (Variables|Propiedades|GetVelocidadEditable)) (Variables|Propiedades|GetFactor)))
  (Utilities|Time|SetTimerbyEvent (delegate Custom|Chequear) (Variables|Propiedades|GetTiempoChequeo) true))

(event Collision|EventActorBeginOverlap
  (params (OtherActor :type Actor%20Object%20Reference)))

(event EventTick
  (params (DeltaSeconds :type Float%20%28single-precision%29))
  (Transformation|AddActorLocalOffset (Variables|Propiedades|GetVelocidad) false false))

(fn ConstructionScript)

(fn SetearEstaSiendoSeguido
  (params (bSeguido :type Boolean))
  (Variables|Propiedades|SetbEstaSiendoSeguido bSeguido))